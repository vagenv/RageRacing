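; Mine actor that detonates when another actor overlaps it, blasting nearby cars and damaging its surroundings.
; On overlap it fires its RadialForce impulse, then loops over all RageBaseCar actors and adds velocity away from the mine to those within PlayerImpulseDistance.
; It then applies radial damage, plays the explosion sound at its location and destroys itself.
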(event `self.ReceiveActorBeginOverlap`
  (params (OtherActor :type "Actor Object Reference"))
  (bind _returnvalue (`self.K2_GetActorLocation`))
  (if (!= OtherActor self)
    (`RadialForceComponent.FireImpulse` (`self.RadialForce`))
    (`|ExecutionSequence`
      (:`then_0`
        (bind _outactors (`GameplayStatics.GetAllActorsOfClass` "/Script/Rage.RageBaseCar"))
        (for _array_element _outactors
          (`/Engine/EditorBlueprintResources/StandardMacros.CompareFloat` (`self.GetDistanceTo` _array_element self) (`self.PlayerImpulseDistance`)
            (:`<`
              (`PrimitiveComponent.SetPhysicsLinearVelocity` (`WheeledVehicle.Mesh` _array_element) (* (`KismetMathLibrary.Normal` (`KismetMathLibrary.GetDirectionVector` (`self.K2_GetActorLocation` self) (`self.K2_GetActorLocation` _array_element))) (`self.PlayerImpulseValue`)) true "None")))))
      (:`then_1`
        (`GameplayStatics.ApplyRadialDamage` :`BaseDamage` (`self.BaseDamage`) :`Origin` _returnvalue :`DamageRadius` (`self.RadialDamage`) :`DamageTypeClass` "/Script/Engine.DamageType" :`DamageCauser` self)
        (`GameplayStatics.PlaySoundAtLocation` "/Game/StarterContent/Audio/Explosion_Cue.Explosion_Cue" _returnvalue))
      (:`then_2`
        (`self.K2_DestroyActor`)))))

(fn `UserConstructionScript`)