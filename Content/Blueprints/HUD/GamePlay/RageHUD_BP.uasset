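; RageHUD_BP is the gameplay HUD Blueprint that creates the main on-screen widget and relays inventory changes to it.
; On BeginPlay it retries on a half-second delay until the owning controller and player are valid.
; It then creates MainWidget_BP, passes it references to the HUD, player and controller, initialises it and adds it to the viewport.
; The InventoryUpdated event tells the widget, if valid, to refresh its inventory.
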(event `self.ReceiveBeginPlay`
  (bind _returnvalue (`self.GetOwningPlayerController`))
  (`/Engine/EditorBlueprintResources/StandardMacros.IsValid` _returnvalue :!label _label
    (:`Is Valid`
      (`/Engine/EditorBlueprintResources/StandardMacros.IsValid` (`self.GetPlayer`) :!label _label_2
        (:`Is Valid`
          (bind _returnvalue_2 (`|CreateWidget` "/Game/Blueprints/HUD/GamePlay/MainWidget_BP.MainWidget_BP_C" _returnvalue))
          (bind _output_get (set `self.MainWidget` _returnvalue_2))
          (set `/Game/Blueprints/HUD/GamePlay/MainWidget_BP.TheHUD` self _output_get)
          (set `/Game/Blueprints/HUD/GamePlay/MainWidget_BP.ThePlayer` (`self.GetPlayer`) _output_get)
          (set `/Game/Blueprints/HUD/GamePlay/MainWidget_BP.TheController` (`self.GetOwningPlayerController`) _output_get)
          (`/Game/Blueprints/HUD/GamePlay/MainWidget_BP.InitialiseWidget_Event` _output_get)
          (`UserWidget.AddToViewport` _output_get 0))
        (:`Is Not Valid`
          (`KismetSystemLibrary.Delay` 0.5)
          (goto _label_2))))
    (:`Is Not Valid`
      (`KismetSystemLibrary.Delay` 0.5)
      (goto _label))))

(event `self.BP_InventoryUpdated`
  (bind _mainwidget (`self.MainWidget`))
  (`/Engine/EditorBlueprintResources/StandardMacros.IsValid` _mainwidget
    (:`Is Valid`
      (`/Game/Blueprints/HUD/GamePlay/MainWidget_BP.UpdateInventory_Event` _mainwidget))))

(fn `UserConstructionScript`)