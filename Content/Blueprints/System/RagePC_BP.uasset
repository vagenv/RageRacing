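; RagePC_BP is a player controller that handles the opening view and spawns the player's car once one is selected.
; On BeginPlay it shows the mouse cursor and sets the view to the first TargetPoint in the level.
; CarSelected_Event spawns PlayerCar_BP just above the first PlayerStart, possesses it and passes the chosen color to the car's material event.
; Some disconnected camera-positioning nodes remain unused.
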(event `self.ReceiveBeginPlay`
  (set `self.bShowMouseCursor` true)
  (bind _outactors (`GameplayStatics.GetAllActorsOfClass` "/Script/Engine.TargetPoint"))
  (bind _item (`KismetArrayLibrary.Array_Get` _outactors))
  (`/Engine/EditorBlueprintResources/StandardMacros.IsValid` _item
    (:`Is Valid`
      (`self.SetViewTargetWithBlend` _item))))

(event `CarSelected_Event`
  (params (CarColor :type "LinearColor Structure"))
  (bind _outactors (`GameplayStatics.GetAllActorsOfClass` "/Script/Engine.PlayerStart"))
  (bind _item (`KismetArrayLibrary.Array_Get` _outactors))
  (`/Engine/EditorBlueprintResources/StandardMacros.IsValid` _item
    (:`Is Valid`
      (bind _returnvalue (`|SpawnActorFromClass` "/Game/Blueprints/System/PlayerCar_BP.PlayerCar_BP_C" (`KismetMathLibrary.MakeTransform` (+ (`self.K2_GetActorLocation` _item) (0.0 0.0 50.0)) (struct)) "Undefined" "OverrideRootScale" self))
      (bind _output_get (set `self.ThePlayer` _returnvalue))
      (`self.Possess` self _output_get)
      (bind _asplayer_car_bp (cast `/Game/Blueprints/System/PlayerCar_BP` _output_get))
      (`/Game/Blueprints/System/PlayerCar_BP.NewCarMaterial_Event` _asplayer_car_bp CarColor))))

(fn `UserConstructionScript`)