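; PlayerCar_BP is the player's car, with camera zoom, an energy-limited boost, recoloring and a flip reset.
; Zoom inputs step the spring arm length within limits.
; Boost runs a timeline that applies forward velocity impulses scaled by current energy while draining it, then restarts energy restore when finished or shortly after depletion.
; Construction creates a dynamic material for color changes, and reset lifts an overturned car upright.
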(event `InputAction|ZoomIn`
  (params (Key :type "Key Structure" :default "AnyKey"))
  (bind _springarm (`self.SpringArm`))
  (bind _returnvalue (- (`SpringArmComponent.TargetArmLength` _springarm) (`self.ZoomRate`)))
  (:`Pressed`
    (if (> _returnvalue (`KismetMathLibrary.BreakVector2D` (`self.MaxCamerZoom`)))
      (set `SpringArmComponent.TargetArmLength` _returnvalue _springarm))))

(event `NewCarMaterial_Event`
  (params (Color :type "LinearColor Structure"))
  (`MaterialInstanceDynamic.SetVectorParameterValue` (`self.CarMaterial`) "Color" Color))

(event `InputAction|ZoomOut`
  (params (Key :type "Key Structure" :default "AnyKey"))
  (bind _springarm (`self.SpringArm`))
  (bind _returnvalue (+ (`SpringArmComponent.TargetArmLength` _springarm) (`self.ZoomRate`)))
  (:`Pressed`
    (if (< _returnvalue (`.Y` (`KismetMathLibrary.BreakVector2D` (`self.MaxCamerZoom`))))
      (set `SpringArmComponent.TargetArmLength` _returnvalue _springarm))))

(event `self.BP_Boost`
  (bind _mesh (`self.Mesh`))
  (bind (_theenergydata_maxvalue _theenergydata_currentvalue _theenergydata_restorespeed _theenergydata_restorevalue _theenergydata_boostmultiplier) (break `EnergyData` (`self.TheEnergyData`)))
  (if (`self.CanBoost`)
    (`|ExecutionSequence`
      (:`then_0`
        (`self.StopEneryRestore`))
      (:`then_1`
        (bind (_direction _boostpower) (`Timeline|BoostTimeline` :!via `PlayFromStart` :!label _label)
          (:`Update`
            (`PrimitiveComponent.AddImpulse` _mesh (* (`SceneComponent.GetForwardVector` _mesh) (* _boostpower _theenergydata_currentvalue _theenergydata_boostmultiplier)) "None" true)
            (`self.UseEnergy` (* _boostpower _theenergydata_maxvalue (`GameplayStatics.GetWorldDeltaSeconds`) 0.5))
            (if (< _theenergydata_currentvalue 1.0)
              (`|ExecutionSequence`
                (:`then_0`
                  (goto _label :!via `Stop`))
                (:`then_1`
                  (`self.UseAllEnergy`))
                (:`then_2`
                  (`KismetSystemLibrary.Delay` 1.0)
                  (`self.StartEneryRestore`)))))
          (:`Finished`
            (`self.StartEneryRestore`)))))))

(event `ResetCar_Event`
  (bind _mesh (`self.Mesh`))
  (if (`self.IsTurnedOver`)
    (`SceneComponent.K2_SetWorldLocationAndRotation` _mesh (+ (`SceneComponent.K2_GetComponentLocation` _mesh) (0.0 0.0 100.0)) (`KismetMathLibrary.MakeRotator` 0.0 (.pitch (`SceneComponent.K2_GetComponentRotation` _mesh)) (.yaw (`SceneComponent.K2_GetComponentRotation` _mesh))) false true)))

(fn `UserConstructionScript`
  (bind _returnvalue (`PrimitiveComponent.CreateDynamicMaterialInstance` (`self.Mesh`) 0 "/Game/Materials/BasicMaterials/BaseMaterial.BaseMaterial"))
  (set `self.CarMaterial` _returnvalue))