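; RageCar_BP is a car Blueprint that handles its chase camera's roll and zoom.
; Each tick, while the mesh roll is under a limit, the camera eases toward a scaled share of that roll, keeping its own pitch and yaw.
; ZoomIn and ZoomOut inputs step the spring arm length within min/max bounds.
; No driving logic appears in these graphs, and BeginPlay only prints a debug string.
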(event `self.ReceiveBeginPlay`
  (`KismetSystemLibrary.PrintString` "my new Car"))

(event `self.ReceiveActorBeginOverlap`
  (params (OtherActor :type "Actor Object Reference")))

(event `self.ReceiveTick`
  (params (DeltaSeconds :type "Float (single-precision)"))
  (bind _camera (`self.Camera`))
  (bind _returnvalue (`SceneComponent.K2_GetComponentRotation` _camera))
  (bind _roll (.roll (`SceneComponent.K2_GetComponentRotation` (`self.Mesh`))))
  (if (< (`KismetMathLibrary.Abs` _roll) (`self.MaxCamerRollAngle`))
    (`SceneComponent.K2_SetWorldRotation` _camera (`KismetMathLibrary.RInterpTo` _returnvalue (`KismetMathLibrary.MakeRot` (.pitch _returnvalue) (.yaw _returnvalue) (* _roll (`self.CameraRollMultiplier`))) DeltaSeconds 1.0) false)))

(event `InputAction|ZoomIn`
  (bind _springarm (`self.SpringArm`))
  (bind _returnvalue (- (`SpringArmComponent.TargetArmLength` _springarm) (`self.ZoomRate`)))
  (:`Pressed`
    (if (> _returnvalue (`KismetMathLibrary.BreakVector2D` (`self.MaxCamerZoom`)))
      (set `SpringArmComponent.TargetArmLength` _returnvalue _springarm))))

(event `InputAction|ZoomOut`
  (bind _springarm (`self.SpringArm`))
  (bind _returnvalue (+ (`SpringArmComponent.TargetArmLength` _springarm) (`self.ZoomRate`)))
  (:`Pressed`
    (if (< _returnvalue (`.Y` (`KismetMathLibrary.BreakVector2D` (`self.MaxCamerZoom`))))
      (set `SpringArmComponent.TargetArmLength` _returnvalue _springarm))))

(fn `UserConstructionScript`)